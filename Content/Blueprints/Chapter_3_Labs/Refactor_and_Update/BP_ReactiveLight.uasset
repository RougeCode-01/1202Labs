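; BP_ReactiveLight is a light actor that reacts to overlaps with its sphere.
; On begin overlap it sets the point light intensity to the ON variable and calls RandomColor for a random RGB color.
; On end overlap it waits OnDuration, then sets the intensity to OFF.
; CheckIfIntensityIsZero runs first on begin overlap, but its zero-intensity branch is empty, so it has no effect.
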(event `self.Sphere.OnComponentBeginOverlap`
  (params (OverlappedComponent :type "PrimitiveComponent Object Reference") (OtherActor :type "Actor Object Reference") (OtherComp :type "PrimitiveComponent Object Reference") (OtherBodyIndex :type Integer) (bFromSweep :type Boolean) (SweepResult :type "HitResult Structure (by ref)"))
  (`self.CheckIfIntensityIsZero`)
  (`LightComponent.SetIntensity` (`self.PointLight`) (`self.ON`))
  (`self.RandomColor`))

(event `self.Sphere.OnComponentEndOverlap`
  (params (OverlappedComponent :type "PrimitiveComponent Object Reference") (OtherActor :type "Actor Object Reference") (OtherComp :type "PrimitiveComponent Object Reference") (OtherBodyIndex :type Integer))
  (`KismetSystemLibrary.Delay` (`self.On Duration`))
  (`LightComponent.SetIntensity` (`self.PointLight`) (`self.OFF`)))

(fn `CheckIfIntensityIsZero`
  (if (== (`LightComponentBase.Intensity` (`self.PointLight`)) 0.0)
    _))

(fn `RandomColor`
  (`LightComponent.SetLightColor` (`self.PointLight`) (`KismetMathLibrary.MakeColor` (`KismetMathLibrary.RandomFloatInRange` 0.0 1.0) (`KismetMathLibrary.RandomFloatInRange` 0.0 1.0) (`KismetMathLibrary.RandomFloatInRange` 0.0 1.0)) true))

(fn `UserConstructionScript`)