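; BP_WorldBounds is an actor whose box marks the playable area, respawning the third-person character when it leaves.
; On end overlap, it destroys any BP_ThirdPersonCharacter exiting the box, waits briefly, then calls Respawn.
; Respawn spawns a fresh character at the location of a PlayerStart found by class, without copying its rotation, and has player controller 0 possess it.
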(event `self.Box.OnComponentEndOverlap`
  (params (OverlappedComponent :type "PrimitiveComponent Object Reference") (OtherActor :type "Actor Object Reference") (OtherComp :type "PrimitiveComponent Object Reference") (OtherBodyIndex :type Integer))
  (bind _asbp_third_person_character (cast `/Game/Blueprints/Chapter_2_Labs/BP_ThirdPersonCharacter` OtherActor))
  (`self.K2_DestroyActor` _asbp_third_person_character)
  (`KismetSystemLibrary.Delay` 0.5)
  (`self.Respawn`))

(fn `Respawn`
  (bind _returnvalue (`GameplayStatics.GetActorOfClass` "/Script/Engine.PlayerStart"))
  (bind _returnvalue_2 (`|SpawnActorFromClass` "/Game/Blueprints/Chapter_2_Labs/BP_ThirdPersonCharacter.BP_ThirdPersonCharacter_C" (`KismetMathLibrary.Conv_VectorToTransform` (`self.K2_GetActorLocation` _returnvalue)) "Undefined" "MultiplyWithRoot" null null))
  (`Controller.Possess` (`GameplayStatics.GetPlayerController` 0) _returnvalue_2))

(fn `UserConstructionScript`)