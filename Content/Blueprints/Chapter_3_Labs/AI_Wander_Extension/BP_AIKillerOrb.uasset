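; AI orb pawn that spots the player and freezes their input on contact.
; PawnSensing sets the SeenPlayer blackboard key when it sees BP_ThirdPersonCharacter.
; Sphere overlap disables that character's input and clears the key; two seconds after overlap ends, input returns, with on-screen messages for both.
; Helper functions wrap blackboard lookup and the cast-guarded input toggles.
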(event `self.PawnSensing.OnSeePawn`
  (params (Pawn :type "Pawn Object Reference"))
  (cast `/Game/Blueprints/Chapter_2_Labs/BP_ThirdPersonCharacter` Pawn)
  (bind _returnvalue (`self.AIController`))
  (`BlackboardComponent.SetValueAsBool` _returnvalue "SeenPlayer" true))

(event `self.Sphere.OnComponentBeginOverlap`
  (params (OverlappedComponent :type "PrimitiveComponent Object Reference") (OtherActor :type "Actor Object Reference") (OtherComp :type "PrimitiveComponent Object Reference") (OtherBodyIndex :type Integer) (bFromSweep :type Boolean) (SweepResult :type "HitResult Structure (by ref)"))
  (`self.DisablePlayerInput` OtherActor)
  (`KismetSystemLibrary.PrintString` "Youve been Frozen" true true (struct :`G` 0.66 :`B` 1.0 :`A` 1.0) 2.0 "1")
  (bind _returnvalue (`self.AIController`))
  (`BlackboardComponent.SetValueAsBool` _returnvalue "SeenPlayer" false))

(event `self.Sphere.OnComponentEndOverlap`
  (params (OverlappedComponent :type "PrimitiveComponent Object Reference") (OtherActor :type "Actor Object Reference") (OtherComp :type "PrimitiveComponent Object Reference") (OtherBodyIndex :type Integer))
  (`KismetSystemLibrary.Delay` 2.0)
  (`self.EnablePlayerInput` OtherActor)
  (`KismetSystemLibrary.PrintString` "Youve been Unfrozen" true true (struct :`G` 0.66 :`B` 1.0 :`A` 1.0) 2.0 "1"))

(fn `AIController`
  (returns (ReturnValue :type "BlackboardComponent Object Reference"))
  (return (`AIBlueprintHelperLibrary.GetBlackboard` (`AIBlueprintHelperLibrary.GetAIController` self))))

(fn `DisablePlayerInput`
  (params (Object :type "Object Object Reference"))
  (bind _asbp_third_person_character (cast `/Game/Blueprints/Chapter_2_Labs/BP_ThirdPersonCharacter` Object))
  (`self.DisableInput` _asbp_third_person_character (`GameplayStatics.GetPlayerController` 0)))

(fn `EnablePlayerInput`
  (params (Object :type "Object Object Reference"))
  (bind _asbp_third_person_character (cast `/Game/Blueprints/Chapter_2_Labs/BP_ThirdPersonCharacter` Object))
  (`self.EnableInput` _asbp_third_person_character (`GameplayStatics.GetPlayerController` 0)))

(fn `UserConstructionScript`)